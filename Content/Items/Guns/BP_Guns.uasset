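; BP_Guns is a gun actor that players can pick up, drop and fire.
; Interaction hands the gun to the player, while a GunState switch toggles physics and collision between on-ground and equipped, starting on the ground.
; Fire spawns an actor at the muzzle socket with velocity toward a distant point along the camera's forward vector, so shots follow the player's aim.
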(event `self.ReceiveBeginPlay`
  (`self.SetGunState` "NewEnumerator0"))

(event `/Game/Blueprints/Interface/InteractionInterface.onInteraction`
  (params (Player :type "/Game/FirstPerson/Blueprints/BP_FirstPersonCharacter Object Reference"))
  (`/Game/FirstPerson/Blueprints/BP_FirstPersonCharacter.Pick Up Gun` Player self)
  (`self.SetGunState` "NewEnumerator1")
  (`SceneComponent.ResetRelativeTransform` (`self.SkeletalMesh`)))

(fn `DroppingGun`
  (`self.SetGunState` "NewEnumerator0"))

(fn `Fire`
  (params (PlayerCamera :type "CameraComponent Object Reference"))
  (bind _returnvalue (`SceneComponent.GetSocketLocation` (`self.SkeletalMesh`) "b_gun_muzzleflash"))
  (`|SpawnActorFromClass` "/Game/Items/BP_Bullet.BP_Bullet_C" (`KismetMathLibrary.MakeTransform` _returnvalue) "Undefined" "OverrideRootScale" null (* (`KismetMathLibrary.Normal` (- (+ (`SceneComponent.K2_GetComponentLocation` PlayerCamera) (* (`SceneComponent.GetForwardVector` PlayerCamera) (100000.0 100000.0 100000.0))) _returnvalue)) (10000.0 10000.0 10000.0)) null))

(fn `GetInteractionText`
  (returns (Text :type Text))
  (return "Pick Up"))

(fn `GetInteractionTextAttached`
  (returns (`Attach Component` :type "SceneComponent Object Reference"))
  (return (`self.SkeletalMesh`)))

(fn `SetGunState`
  (params (NewGunState :type "/Game/Items/Guns/E_GunState Enum" :default "NewEnumerator0"))
  (bind _skeletalmesh (`self.SkeletalMesh`))
  (bind _skeletalmesh_2 (`self.SkeletalMesh`))
  (bind _output_get (set `self.Gun State` NewGunState))
  (switch `/Game/Items/Guns/E_GunState` _output_get
    (:`NewEnumerator0`
      (`PrimitiveComponent.SetCollisionProfileName` (`self.Sphere`) "OverlapAllDynamic" true)
      (`PrimitiveComponent.SetSimulatePhysics` _skeletalmesh_2 true)
      (`PrimitiveComponent.SetCollisionProfileName` _skeletalmesh_2 "DroppedGun" true))
    (:`NewEnumerator1`
      (`PrimitiveComponent.SetCollisionProfileName` (`self.Sphere`) "NoCollision" true)
      (`PrimitiveComponent.SetSimulatePhysics` _skeletalmesh false)
      (`PrimitiveComponent.SetCollisionProfileName` _skeletalmesh "NoCollision" true))))

(fn `UserConstructionScript`
  (`parent.UserConstructionScript`))